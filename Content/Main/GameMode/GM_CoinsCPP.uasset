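; GM_CoinsCPP is a game mode Blueprint that drives the HUD for a timed coin-collecting objective.
; On BeginPlay it creates WP_GoldenHud, adds it to the viewport, and fills in the coins-needed and coins-gathered text.
; Small update functions copy CoinsNeededCPP, CoinsGhateredCPP and TimeRemaining into the widget's text fields.
; TimerUpdate has no caller in this graph, and neither the countdown nor coin counting happens here.
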(event `self.ReceiveBeginPlay`
  (bind _returnvalue (`|CreateWidget` "/Game/Main/Hud/WP_GoldenHud.WP_GoldenHud_C"))
  (set `self.GoldenHudRef` _returnvalue)
  (`UserWidget.AddToViewport` (`self.GoldenHudRef`) 0)
  (`self.CoinsNeededHud`)
  (`self.CoinsGhateredUpdate`))

(fn `CoinsGhateredUpdate`
  (`TextBlock.SetText` (`/Game/Main/Hud/WP_GoldenHud.CoinsGhateredHud` (`self.GoldenHudRef`)) (`KismetTextLibrary.Conv_IntToText` (`self.CoinsGhateredCPP`)))
  (return))

(fn `CoinsNeededHud`
  (`TextBlock.SetText` (`/Game/Main/Hud/WP_GoldenHud.CoisNeedToWin` (`self.GoldenHudRef`)) (`KismetTextLibrary.Conv_IntToText` (`self.CoinsNeededCPP`))))

(fn `TimerUpdate`
  (`TextBlock.SetText` (`/Game/Main/Hud/WP_GoldenHud.TimerHudText` (`self.GoldenHudRef`)) (`KismetTextLibrary.Conv_IntToText` (`self.TimeRemaining`)))
  (return))

(fn `UserConstructionScript`)