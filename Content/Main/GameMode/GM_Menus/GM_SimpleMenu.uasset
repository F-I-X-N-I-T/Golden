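; GM_SimpleMenu is a game mode for a simple menu screen.
; On BeginPlay it creates the WBP_MenuSimple widget, adds it to the viewport and starts the SC_GameLevel sound in 2D, keeping references to both.
; It binds to the widget's new-level press event, which fades the sound out.
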(event `self.ReceiveBeginPlay`
  (bind _returnvalue (`|CreateWidget` "/Game/Main/Hud/Menu/WBP_MenuSimple.WBP_MenuSimple_C"))
  (set `self.WidgetRef` _returnvalue)
  (`UserWidget.AddToViewport` (`self.WidgetRef`) 0)
  (add `/Game/Main/Hud/Menu/WBP_MenuSimple.OnNewLevelPress` (`self.WidgetRef`) (delegate `OnNewLevelPress`))
  (bind _returnvalue_2 (`GameplayStatics.SpawnSound2D` "/Game/Main/Sounds/GoldenHunt/Environment/SC_GameLevel.SC_GameLevel" 1.0 1.0 0.0 null))
  (set `self.SoundRef` _returnvalue_2))

(event `OnNewLevelPress`
  (`AudioComponent.FadeOut` (`self.SoundRef`) 0.75 0.0 "Linear"))

(fn `UserConstructionScript`)