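; GM_Coins is a game mode Blueprint containing a simple countdown timer built on a looping timer handle.
; TimerEvent decrements Counter and clears the timer once it reaches CounterStopTimer.
; The nodes that create the timer and print the counter are disconnected, and BeginPlay and Tick are empty, so nothing in this graph starts the countdown.
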(event `self.ReceiveBeginPlay`)

(event `TimerEvent`
  ; TimerCount and Clear Timer
  (bind _result (`/Engine/EditorBlueprintResources/StandardMacros.DecrementInt` (`self.Counter`))
    (:`  `
      (if (<= _result (`self.CounterStopTimer`))
        (`KismetSystemLibrary.K2_ClearAndInvalidateTimerHandle` (`self.SetTimerByEvent`))))))

(event `self.ReceiveTick`
  (params (DeltaSeconds :type "Float (single-precision)")))

(fn `UserConstructionScript`)