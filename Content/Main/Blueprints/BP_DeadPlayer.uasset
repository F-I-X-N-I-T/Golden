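; BP_DeadPlayer is a box trigger volume that sends the player back to a spawn point, apparently as a death or kill zone.
; When an overlapping actor has the PlayerA1 tag, it is moved without sweep to the location of the referenced SpawnActor, with only its location set.
; The construction script sizes the box from the BoxSize variable.
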(event `self.ReceiveActorBeginOverlap`
  (params (OtherActor :type "Actor Object Reference"))
  (set `self.Other Actor` OtherActor)
  (if (`self.ActorHasTag` (`self.Other Actor`) "PlayerA1")
    (`self.K2_SetActorLocation` (`self.Other Actor`) (`self.K2_GetActorLocation` (`self.SpawnActor`)) false false)))

(fn `UserConstructionScript`
  (`BoxComponent.SetBoxExtent` (`self.Box`) (`self.BoxSize`) true))